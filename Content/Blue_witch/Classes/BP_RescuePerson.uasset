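; BP_RescuePerson is a Paper2D character that, by its name, is a person to rescue, carrying what looks like copied player-mage logic.
; Its events are empty and the animation, firing, hit/knockback, movement and HUD chains are disconnected, so none run.
; The unused functions pick eight-direction flipbooks from movement or hardcoded screen-space cursor zones, and add health widgets, playing a death flipbook at zero.
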(event EventBeginPlay)

(event Collision|EventActorBeginOverlap
  (params (OtherActor :type Actor%20Object%20Reference)))

(event EventTick
  (params (DeltaSeconds :type Float%20%28single-precision%29))
  ;[1 1 1] Animations and HUD
)

(fn ConstructionScript)

(fn Animate
  (bind _animations (Variables|Default|GetAnimations))
  (LocalVariables|SetLocalUpOrDown (Input|AxisValues|GetMoveForward/Backward))
  (LocalVariables|SetLocalLeftOrRight (Input|AxisValues|GetMoveRight/Left))
  ;[1 1 1] Are we moving?
  (if (or (!= (LocalVariables|GetLocalUpOrDown) 0.0) (!= (LocalVariables|GetLocalLeftOrRight) 0.0))
    (Variables|Default|SetMoveDirection (select (and (> (LocalVariables|GetLocalUpOrDown) 0.0) (< (Math|Float|Absolute(Float) (LocalVariables|GetLocalLeftOrRight)) 0.5)) "NewEnumerator0" (select (and (> (LocalVariables|GetLocalUpOrDown) 0.5) (> (LocalVariables|GetLocalLeftOrRight) 0.5)) "NewEnumerator5" (select (and (> (LocalVariables|GetLocalUpOrDown) 0.5) (< (LocalVariables|GetLocalLeftOrRight) -0.5)) "NewEnumerator4" (select (and (< (LocalVariables|GetLocalUpOrDown) -0.5) (< (Math|Float|Absolute(Float) (LocalVariables|GetLocalLeftOrRight)) 0.5)) "NewEnumerator1" (select (and (< (LocalVariables|GetLocalUpOrDown) -0.5) (> (LocalVariables|GetLocalLeftOrRight) 0.5)) "NewEnumerator7" (select (and (< (LocalVariables|GetLocalUpOrDown) -0.5) (< (LocalVariables|GetLocalLeftOrRight) -0.5)) "NewEnumerator6" (select (and (< (Math|Float|Absolute(Float) (LocalVariables|GetLocalUpOrDown)) 0.5) (> (LocalVariables|GetLocalLeftOrRight) 0.0)) "NewEnumerator3" "NewEnumerator2")))))))))
  (Sprite|SetFlipbook (Variables|Default|GetSprite) (select (> (Math|Vector|VectorLength (Transformation|GetVelocity)) 0.0) (Utilities|Select :Index (Variables|Default|GetMoveDirection) :NewEnumerator0 (.walkup _animations) :NewEnumerator1 (.walkdown _animations) :NewEnumerator2 (.walkleft _animations) :NewEnumerator3 (.walkright _animations) :NewEnumerator4 (.walkul _animations) :NewEnumerator5 (.walkur _animations) :NewEnumerator6 (.walkdl _animations) :NewEnumerator7 (.walkdr _animations)) (Utilities|Select :Index (Variables|Default|GetMoveDirection) :NewEnumerator0 (.idleup _animations) :NewEnumerator1 (.idledown _animations) :NewEnumerator2 (.idleleft _animations) :NewEnumerator3 (.idleright _animations) :NewEnumerator4 (.idleul _animations) :NewEnumerator5 (.idleur _animations) :NewEnumerator6 (.idledl _animations) :NewEnumerator7 (.idledr _animations)))))

(fn AnimateAttack
  (bind _atkanimation (Variables|Default|GetAtkAnimation))
  (bind _atkanimation_2 (Variables|Default|GetAtkAnimation))
  ;[1 1 1] MIT MOUSE DIRECTION ARBEITEN
  (bind _returnvalue (Class|WidgetLayoutLibrary|GetMousePositiononViewport))
  (Development|PrintString (Utilities|String|ToString(Vector2d) _returnvalue))
  (bind _returnvalue_2 (Class|WidgetLayoutLibrary|GetMousePositiononViewport))
  (Variables|Default|SetX (.x _returnvalue_2))
  (Variables|Default|SetY (.y _returnvalue_2))
  (LocalVariables|SetLocalUpOrDown2 (Input|AxisValues|GetMoveForward/Backward))
  (LocalVariables|SetLocalLeftOrRight2 (Input|AxisValues|GetMoveRight/Left))
  ;[1 1 1] Are we moving?
  (if true
    (Development|PrintString "Hello")
    (Variables|Default|SetMoveDirection (select (and (< (Variables|Default|GetY) 5.9e+02) (and (> (Variables|Default|GetX) 875.0) (< (Variables|Default|GetX) 1e+03))) "NewEnumerator0" (select (and (> (Variables|Default|GetY) 5.9e+02) (and (> (Variables|Default|GetX) 875.0) (< (Variables|Default|GetX) 1e+03))) "NewEnumerator1" (select (and (< (Variables|Default|GetX) 933.0) (and (< (Variables|Default|GetY) 6.7e+02) (> (Variables|Default|GetY) 5.3e+02))) "NewEnumerator2" (select (and (> (Variables|Default|GetX) 933.0) (and (< (Variables|Default|GetY) 6.7e+02) (> (Variables|Default|GetY) 5.3e+02))) "NewEnumerator3" (select (and (> (Variables|Default|GetX) 1e+03) (> (Variables|Default|GetY) 6.7e+02)) "NewEnumerator7" (select (and (< (Variables|Default|GetX) 1e+03) (> (Variables|Default|GetY) 6.7e+02)) "NewEnumerator6" (select (and (> (Variables|Default|GetX) 1e+03) (< (Variables|Default|GetY) 5.2e+02)) "NewEnumerator5" "NewEnumerator4")))))))))
  (Sprite|SetFlipbook (Variables|Default|GetSprite) (select (> (Math|Vector|VectorLength (Transformation|GetVelocity)) 0.0) (Utilities|Select :Index (Variables|Default|GetMoveDirection) :NewEnumerator0 (.atkup _atkanimation) :NewEnumerator1 (.atkdown _atkanimation) :NewEnumerator2 (.atkleft _atkanimation) :NewEnumerator3 (.atkright _atkanimation) :NewEnumerator4 (.atkul _atkanimation) :NewEnumerator5 (.atkur _atkanimation) :NewEnumerator6 (.atkdl _atkanimation) :NewEnumerator7 (.atkdr _atkanimation)) (Utilities|Select :Index (Variables|Default|GetMoveDirection) :NewEnumerator0 (.atkup _atkanimation_2) :NewEnumerator1 (.atkdown _atkanimation_2) :NewEnumerator2 (.atkleft _atkanimation_2) :NewEnumerator3 (.atkright _atkanimation_2) :NewEnumerator4 (.atkul _atkanimation_2) :NewEnumerator5 (.atkur _atkanimation_2) :NewEnumerator6 (.atkdl _atkanimation_2) :NewEnumerator7 (.atkdr _atkanimation_2)))))

(fn CheckHealthbar
  (if (== (Variables|Default|GetHealth) 3.0)
    (bind _returnvalue (UserInterface|CreateWidget "/Game/Blue_witch/Heart_Hud/W_PlayerHub_3.W_PlayerHub_3_C" (Game|GetPlayerController 0)))
    (UserInterface|Viewport|AddtoViewport _returnvalue 0)
    (elif (== (Variables|Default|GetHealth) 2.0)
      (bind _returnvalue_2 (UserInterface|CreateWidget "/Game/Blue_witch/Heart_Hud/W_PlayerHub_2.W_PlayerHub_2_C" (Game|GetPlayerController 0)))
      (UserInterface|Viewport|AddtoViewport _returnvalue_2 0)
      (elif (== (Variables|Default|GetHealth) 1.0)
        (bind _returnvalue_3 (UserInterface|CreateWidget "/Game/Blue_witch/Heart_Hud/W_PlayerHub_1.W_PlayerHub_1_C" (Game|GetPlayerController 0)))
        (UserInterface|Viewport|AddtoViewport _returnvalue_3 0)
        (elif (< (Variables|Default|GetHealth) 1.0)
          (bind _returnvalue_4 (UserInterface|CreateWidget "/Game/Blue_witch/Heart_Hud/W_PlayerHub_0.W_PlayerHub_0_C" (Game|GetPlayerController 0)))
          (UserInterface|Viewport|AddtoViewport _returnvalue_4 0)
          (CallFunction|HeroDie))))))

(fn HeroDie
  (Sprite|SetFlipbook (Variables|Default|GetSprite) "/Game/Blue_witch/NewChar/Sprites/Mage_die.Mage_die"))