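; Fire projectile in the Blue_witch folder that plays a fireball sound on spawn and destroys itself after a short lifetime.
; On hit, actors tagged enemy or dummy are cast to GreenSlime, which loses Damage health and is marked not alive at zero or below.
; The projectile is destroyed on slime or untagged hits; tagged non-slime actors take no damage and do not destroy it.
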(event Collision|EventActorBeginOverlap
  (params (OtherActor :type Actor%20Object%20Reference)))

(event EventTick
  (params (DeltaSeconds :type Float%20%28single-precision%29)))

(event EventBeginPlay
  (Audio|PlaySound2D "/Game/Audio/431174__highpixel__fireball-explosion.431174__highpixel__fireball-explosion" 1.0 1.0 0.0 0 0)
  (Utilities|FlowControl|Delay 1.5)
  (Actor|DestroyActor))

(event Collision|EventHit
  (params (MyComp :type Primitive%20Component%20Object%20Reference) (Other :type Actor%20Object%20Reference) (OtherComp :type Primitive%20Component%20Object%20Reference) (bSelfMoved :type Boolean) (HitLocation :type Vector :default "0, 0, 0") (HitNormal :type Vector :default "0, 0, 0") (NormalImpulse :type Vector :default "0, 0, 0") (Hit :type Hit%20Result%20Structure%20%28by%20ref%29))
  (bind _hitactor (Collision|BreakHitResult Hit))
  (bind _returnvalue (Actor|ActorHasTag _hitactor "enemy"))
  (bind _returnvalue_2 (Actor|ActorHasTag _hitactor "dummy"))
  (Utilities|FlowControl|Sequence
    (:then_0
      (if (or _returnvalue _returnvalue_2)
        (bind _asgreen_slime (Utilities|Casting|CastToGreenSlime Other))
        (bind _output_get (Variables|/Game/Slime/GreenSlime.GreenSlime_C|SetHealthSlime _asgreen_slime (- (Variables|/Game/Slime/GreenSlime.GreenSlime_C|GetHealthSlime _asgreen_slime) (Variables|Default|GetDamage))))
        (Actor|DestroyActor)
        (if (and (<= _output_get 0.0) (or _returnvalue _returnvalue_2))
          (Variables|/Game/Slime/GreenSlime.GreenSlime_C|SetAlive _asgreen_slime false))))
    (:then_1
      (if (not (or _returnvalue _returnvalue_2))
        (Actor|DestroyActor)))))

(fn ConstructionScript)